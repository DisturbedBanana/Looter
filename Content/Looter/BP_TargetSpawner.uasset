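; BP_TargetSpawner is an actor that keeps its list of BP_Target actors topped up to a maximum count.
; On Tick, while below the limit, it spawns one target, sets itself as that target's Parent and adds it to TargetsList.
; Helper functions randomize each spawn point around the spawner: symmetric in X, only toward negative Y, and within a min/max Z offset.
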(event EventTick
  (params (DeltaSeconds :type Float%20%28single-precision%29))
  (if (< (Utilities|Array|Length (Variables|Default|GetTargetsList)) (Variables|Default|GetMaxTargetNumber))
    (bind _returnvalue (Game|SpawnActorfromClass "/Game/Looter/BP_Target.BP_Target_C" (Math|Transform|MakeTransform (CallFunction|AddRandomPosition (Transformation|GetActorLocation) 5.0 5.0 2.0 6.0) "0, 0, 0" "1.000000,1.000000,1.000000") "Undefined" "MultiplyWithRoot" 0 0))
    (Variables|/Game/Looter/BP_Target.BP_Target_C|Setparent _returnvalue self)
    (Utilities|Array|Add (Variables|Default|GetTargetsList) _returnvalue)))

(fn ConstructionScript)

(fn AddRandomPosition
  (params (Base%20position :type Vector) (X%20range :type Float%20%28double-precision%29) (Y%20range :type Float%20%28double-precision%29) (Z%20min :type Float%20%28double-precision%29) (Z%20max :type Float%20%28double-precision%29))
  (return (Math|Vector|MakeVector (|randomX (.x Base%20position) X%20range) (|randomY (.y Base%20position) Y%20range) (|randomZ (.z Base%20position) Z%20min Z%20max))))